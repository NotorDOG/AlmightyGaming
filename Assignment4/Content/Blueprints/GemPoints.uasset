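; GemPoints is a collectible gem actor that adds points to the player when the AlmightyPawn hits it.
; The construction script uses the Gem type to set the mesh material color and a matching GemValue.
; On hit, it passes GemValue to AlmightyController's AddGem and destroys itself.
; Tick bobs the mesh vertically with a sine of game time.
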(event `self.ReceiveHit`
  (params (MyComp :type "PrimitiveComponent Object Reference") (Other :type "Actor Object Reference") (OtherComp :type "PrimitiveComponent Object Reference") (bSelfMoved :type Boolean) (HitLocation :type "Vector Structure") (HitNormal :type "Vector Structure") (NormalImpulse :type "Vector Structure") (Hit :type "HitResult Structure (by ref)"))
  (cast `/Game/Blueprints/Player/AlmightyLevel/AlmightyPawn` Other)
  (bind _asalmighty_controller (cast `/Game/Blueprints/Player/AlmightyLevel/AlmightyController` (`GameplayStatics.GetPlayerController` 0)))
  (`/Game/Blueprints/Player/AlmightyLevel/AlmightyController.AddGem` _asalmighty_controller (`self.GemValue`))
  (`self.K2_DestroyActor`))

(event `self.ReceiveTick`
  (params (DeltaSeconds :type "Float (single-precision)"))
  (`SceneComponent.K2_SetRelativeLocation` (`self.Mesh`) (`KismetMathLibrary.MakeVector` 0.0 0.0 (* (`KismetMathLibrary.Sin` (* 5 (`KismetSystemLibrary.GetGameTimeInSeconds`))) 10.0)) false false))

(fn `UserConstructionScript`
  (bind _mesh (`self.Mesh`))
  (switch `/Game/Blueprints/GemKinds` (`self.Gem`)
    (:`NewEnumerator0`
      (`PrimitiveComponent.SetMaterial` _mesh 0 "/Game/MundellsStarterContent/Materials/Red.Red")
      (set `self.GemValue` 1))
    (:`NewEnumerator1`
      (`PrimitiveComponent.SetMaterial` _mesh 0 "/Game/MundellsStarterContent/Materials/Yellow.Yellow")
      (set `self.GemValue` 2))
    (:`NewEnumerator2`
      (`PrimitiveComponent.SetMaterial` _mesh 0 "/Game/MundellsStarterContent/Materials/Cyan.Cyan")
      (set `self.GemValue` 3))
    (:`NewEnumerator3`
      (`PrimitiveComponent.SetMaterial` _mesh 0 "/Game/MundellsStarterContent/Materials/Magenta.Magenta")
      (set `self.GemValue` 4))
    (:`NewEnumerator4`
      (`PrimitiveComponent.SetMaterial` _mesh 0 "/Game/MundellsStarterContent/Materials/Green.Green")
      (set `self.GemValue` 5))))